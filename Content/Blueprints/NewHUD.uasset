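; NewHUD is an actor that puts two screen widgets, a main screen and an advanced view, on the player's screen.
; On BeginPlay it adds both widgets from its widget components, showing the main one and hiding the advanced one.
; SwitchHUDs checks each widget's visibility but, as wired, re-applies the current state instead of toggling it.
; An unconnected chain that would deactivate both screens never runs.
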(event `self.ReceiveBeginPlay`
  (bind _returnvalue (`WidgetComponent.GetUserWidgetObject` (`self.WidgetMain`)))
  (bind _returnvalue_2 (`WidgetComponent.GetUserWidgetObject` (`self.WidgetAdvView`)))
  (`UserWidget.AddToPlayerScreen` _returnvalue 0)
  (`UserWidget.AddToPlayerScreen` _returnvalue_2 0)
  (`Widget.SetVisibility` _returnvalue_2 "Hidden")
  (`Widget.SetVisibility` _returnvalue "Visible"))

(fn `SwitchHUDs`
  (bind _returnvalue (`WidgetComponent.GetUserWidgetObject` (`self.WidgetMain`)))
  (bind _returnvalue_2 (`WidgetComponent.GetUserWidgetObject` (`self.WidgetAdvView`)))
  (if (not (`Widget.IsVisible` _returnvalue))
    (`Widget.SetVisibility` _returnvalue "Hidden")
    (else
      (`Widget.SetVisibility` _returnvalue "Visible")))
  (if (not (`Widget.IsVisible` _returnvalue_2))
    (`Widget.SetVisibility` _returnvalue_2 "Hidden")
    (else
      (`Widget.SetVisibility` _returnvalue_2 "Visible"))))

(fn `UserConstructionScript`)